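; BP_Transport is a level exit that sends the hero on to a new level.
; Both the box overlap and the Interacted event call Transport, which destroys the box before checking for a BdCharacterHero.
; For a hero, it plays an explosion sound and asks BulletDungeonGameModeBase to load and travel to the new level.
; Tick keeps the actor yawed along the direction from the player pawn to itself.
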(event OnComponentBeginOverlap(Box)
  (params (OverlappedComponent :type Primitive%20Component%20Object%20Reference) (OtherActor :type Actor%20Object%20Reference) (OtherComp :type Primitive%20Component%20Object%20Reference) (OtherBodyIndex :type Integer) (bFromSweep :type Boolean) (SweepResult :type Hit%20Result%20Structure%20%28by%20ref%29))
  (CallFunction|Transport OtherActor))

(event EventBeginPlay)

(event Collision|EventActorBeginOverlap
  (params (OtherActor :type Actor%20Object%20Reference)))

(event EventTick
  (params (DeltaSeconds :type Float%20%28single-precision%29))
  (Transformation|SetActorRotation (Math|Rotator|MakeRotator 0.0 0.0 (.Yaw (Math|Rotator|BreakRotator (Math|Conversions|RotationFromXVector (- (Transformation|GetActorLocation) (Transformation|GetActorLocation (Game|Player|GetPlayerPawn 0)))))))))

(event EventInteracted
  (params (InstigatorPawn :type Pawn%20Object%20Reference))
  (CallFunction|Transport (stale OnComponentBeginOverlap(Box) OtherActor)))

(fn ConstructionScript)

(fn Transport
  (params (Insighter :type Actor%20Object%20Reference))
  (Components|DestroyComponent (Variables|Default|GetBox))
  (Utilities|Casting|CastToBdCharacterHero Insighter)
  (Audio|PlaySound2D "/Game/Environment/Sound/Explosion01.Explosion01" 1.0 1.0 0.0 0 0)
  (bind _asbullet_dungeon_game_mode_base (Utilities|Casting|CastToBulletDungeonGameModeBase (Game|GetGameMode)))
  (Class|BulletDungeonGameModeBase|LoadandTravelNewLevel _asbullet_dungeon_game_mode_base))