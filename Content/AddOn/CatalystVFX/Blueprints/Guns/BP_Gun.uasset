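; Base first-person gun in the CatalystVFX add-on that binds to the player character's trigger and equip events, leaving firing behavior to child Blueprints.
; Trigger pulls call the empty FireSequence event, gated by a cooldown.
; Equipping plays a timeline that animates mask and emissive parameters on a color-tinted dynamic material.
; Helper functions trace within a spread cone, from screen center or muzzle, returning aimed spawn transforms and hit data.
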(event Custom|ListenerEquippedWeapon
  (bind _gundmi (Variables|Default|GetGunDMI))
  (bind _newtrack_0 (Timeline|Timeline_0 PlayFromStart)
    (:Update
      (Rendering|Material|SetScalarParameterValue _gundmi "MaskTransition" _newtrack_0 :!class /Script/Engine.MaterialInstanceDynamic)
      (Rendering|Material|SetScalarParameterValue _gundmi "FullEmissive" (Math|Float|Lerp 1.0 0.0 _newtrack_0) :!class /Script/Engine.MaterialInstanceDynamic))))

(event Custom|TriggerPull
  (if (not (Variables|Default|GetIsOnCooldown))
    (Variables|Default|SetIsOnCooldown true)
    (CallFunction|FireSequence)
    (Utilities|FlowControl|Delay (Variables|Default|GetCooldown))
    (Variables|Default|SetIsOnCooldown false)))

(event Custom|FireSequence
  ;[1 1 1] Event to be used with child blueprints
)

(event Custom|TriggerReleased
  ;[1 1 1] Used with child widgets
)

(event EventBeginPlay
  (bind _asbp_first_person_character (Utilities|Casting|CastToBP_FirstPersonCharacter (Game|GetPlayerCharacter 0)))
  (bind _output_get (Variables|Default|SetPlayerCharacter _asbp_first_person_character))
  (EventDispatchers|BindEventtoTriggerPull _output_get (delegate Custom|TriggerPull))
  (EventDispatchers|BindEventtoTriggerRelease _output_get (delegate Custom|TriggerReleased))
  (EventDispatchers|BindEventtoEquippedWeapon _output_get (delegate Custom|ListenerEquippedWeapon)))

(event Collision|EventActorBeginOverlap
  (params (OtherActor :type Actor%20Object%20Reference)))

(event EventTick
  (params (DeltaSeconds :type Float%20%28single-precision%29)))

(fn ConstructionScript
  (bind _returnvalue (Rendering|Material|CreateDynamicMaterialInstance (Variables|Default|GetSK_FPGun) 0 0 "None" :!class /Script/Engine.PrimitiveComponent))
  (bind _output_get (Variables|Default|SetGunDMI _returnvalue))
  (Rendering|Material|SetVectorParameterValue _output_get "BodyColor" (Math|Conversions|ToLinearColor(Color) (Variables|Default|GetColor)) :!class /Script/Engine.MaterialInstanceDynamic))

(fn GetProjectileTarget
  (params (Distance :type Float%20%28double-precision%29) (Offset :type Vector%202D%20Structure))
  (bind _playercharacter (Variables|Default|GetPlayerCharacter))
  (bind _playercharacter_2 (Variables|Default|GetPlayerCharacter))
  (bind _firstpersoncamera (Variables|/Game/AddOn/CatalystVFX/Blueprints/BP_FirstPersonCharacter.BP_FirstPersonCharacter_C|GetFirstPersonCamera _playercharacter))
  (bind _firstpersoncamera_2 (Variables|/Game/AddOn/CatalystVFX/Blueprints/BP_FirstPersonCharacter.BP_FirstPersonCharacter_C|GetFirstPersonCamera _playercharacter_2))
  (bind _gunoffset (Variables|/Game/AddOn/CatalystVFX/Blueprints/BP_FirstPersonCharacter.BP_FirstPersonCharacter_C|GetGunOffset _playercharacter))
  (bind _arrow1 (Variables|/Game/AddOn/CatalystVFX/Blueprints/BP_FirstPersonCharacter.BP_FirstPersonCharacter_C|GetArrow1 _playercharacter))
  (bind _returnvalue (Transformation|GetWorldTransform _arrow1))
  (bind _returnvalue_2 (Transformation|GetWorldRotation _firstpersoncamera))
  (bind _returnvalue_3 (Transformation|GetWorldLocation _firstpersoncamera_2))
  (bind _returnvalue_4 (Math|Vector|RotateVector _gunoffset _returnvalue_2))
  (bind _returnvalue_5 (+ (.location _returnvalue) _returnvalue_4))
  (bind _outhit (Collision|LineTraceByChannel _returnvalue_3 (+ (* (Math|Random|RandomUnitVectorinConeinDegrees (.WorldDirection (Class|GameplayStatics|DeprojectScreentoWorld (Game|GetPlayerController 0) (+ (/ (Viewport|GetViewportSize) 2.0) Offset))) (Variables|Default|GetSpread)) Distance) _returnvalue_3) "TraceTypeQuery1" false 0 "None"))
  (return (select (.bBlockingHit (Collision|BreakHitResult _outhit)) (Math|Transform|MakeTransform _returnvalue_5 (Math|Rotator|FindLookatRotation _returnvalue_5 (.ImpactPoint (Collision|BreakHitResult _outhit)))) (Math|Transform|MakeTransform _returnvalue_5 (Math|Rotator|FindLookatRotation _returnvalue_5 (.TraceEnd (Collision|BreakHitResult _outhit))))) (.TraceEnd (Collision|BreakHitResult _outhit)) (.bBlockingHit (Collision|BreakHitResult _outhit)) (.ImpactPoint (Collision|BreakHitResult _outhit)) (.ImpactNormal (Collision|BreakHitResult _outhit))))

(fn GetAutoTarget
  (params (Distance :type Float%20%28double-precision%29))
  (bind _muzzleflash (Variables|Default|GetMuzzleFlash))
  (bind _muzzleflash_2 (Variables|Default|GetMuzzleFlash))
  (bind _returnvalue (Transformation|GetWorldLocation _muzzleflash))
  (bind _returnvalue_2 (Transformation|GetWorldLocation _muzzleflash_2))
  (bind _outhit (Collision|LineTraceByChannel _returnvalue_2 (+ (* (Math|Random|RandomUnitVectorinConeinDegrees (Math|Vector|GetForwardVector (Variables|Default|GetMuzzleFlash)) (Variables|Default|GetSpread)) Distance) _returnvalue_2) "TraceTypeQuery1" false 0 "None"))
  (return (select (.bBlockingHit (Collision|BreakHitResult _outhit)) (Math|Transform|MakeTransform _returnvalue (Math|Rotator|FindLookatRotation _returnvalue (.ImpactPoint (Collision|BreakHitResult _outhit)))) (Math|Transform|MakeTransform _returnvalue (Math|Rotator|FindLookatRotation _returnvalue (.TraceEnd (Collision|BreakHitResult _outhit))))) (.TraceEnd (Collision|BreakHitResult _outhit)) (.bBlockingHit (Collision|BreakHitResult _outhit)) (.ImpactPoint (Collision|BreakHitResult _outhit)) (.ImpactNormal (Collision|BreakHitResult _outhit))))