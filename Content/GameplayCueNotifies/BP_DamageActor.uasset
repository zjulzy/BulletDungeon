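; BP_DamageActor is a floating damage number actor that shows a damage value, drifts and then removes itself.
; On Activate, it passes its Damage value to the BP_DamageUI widget held by its widget component.
; A timeline then lerps the actor from its current location to a fixed, raised world-space offset and destroys it on finish.
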(event Custom|Activate
  (bind _asbp_damage_ui (Utilities|Casting|CastToBP_DamageUI (UserInterface|GetWidget (Variables|Default|GetWidget))))
  (Variables|/Game/GameplayCueNotifies/BP_DamageUI.BP_DamageUI_C|SetDamage _asbp_damage_ui (Variables|Default|GetDamage))
  (bind _output_get (Variables|Default|SetStartLoc (Transformation|GetActorLocation)))
  (Variables|Default|SetEndLoc (+ _output_get "25.000000,-25.000000,50.000000"))
  (bind _newtrack_0 (Timeline|Timeline Play)
    (:Update
      (Transformation|SetActorLocation (Math|Vector|Lerp(Vector) (Variables|Default|GetStartLoc) (Variables|Default|GetEndLoc) _newtrack_0) false false))
    (:Finished
      (Actor|DestroyActor))))

(fn ConstructionScript)