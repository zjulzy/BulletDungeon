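; Gameplay ability for automatic rifle fire that repeatedly triggers single-shot attacks while the input is held.
; A looping timer, paced by the hero main weapon's ShootSpeed with a negative start delay for an immediate first shot, activates abilities tagged Ability.Weapon.Rifle.SingleAttack.
; Releasing input ends the ability, which pauses the timer; later activations resume that stored timer while its handle stays valid, rather than creating another.
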(event Custom|Fire
  (Abilities|TryActivateAbilitiesbyTag (.AbilitySystemComponent (Utilities|Struct|BreakGameplayAbilityActorInfo (Ability|GetActorInfo))) (GameplayTags|MakeGameplayTagContainerfromTag "(TagName=\"Ability.Weapon.Rifle.SingleAttack\")") true))

(event Ability|EventOnEndAbility
  (params (bWasCancelled :type Boolean))
  (Development|PrintString "end attack ability")
  (Utilities|Time|PauseTimerbyHandle (Variables|Default|GetTH_Shoot)))

(event Ability|EventActivateAbility
  (Ability|Tasks|WaitInputRelease true
    (:then
      (Development|PrintString "activate fire")
      (if (Utilities|Time|IsValidTimerHandle (Variables|Default|GetTH_Shoot))
        (Utilities|Time|UnpauseTimerbyHandle (Variables|Default|GetTH_Shoot))
        (else
          (bind _asbd_character_hero (Utilities|Casting|CastToBdCharacterHero (.AvatarActor (Utilities|Struct|BreakGameplayAbilityActorInfo (Ability|GetActorInfo)))))
          (bind _returnvalue (Utilities|Time|SetTimerbyEvent (delegate Custom|Fire) (Variables|/Script/BulletDungeon.BdWeaponBase|GetShootSpeed (Variables|/Script/BulletDungeon.BdCharacterHero|GetMainWeapon _asbd_character_hero)) true (* (Variables|/Script/BulletDungeon.BdWeaponBase|GetShootSpeed (Variables|/Script/BulletDungeon.BdCharacterHero|GetMainWeapon _asbd_character_hero)) -1.0)))
          (Variables|Default|SetTH_Shoot _returnvalue))))
    (:OnRelease
      (Development|PrintString "release attack")
      (Ability|EndAbility))))