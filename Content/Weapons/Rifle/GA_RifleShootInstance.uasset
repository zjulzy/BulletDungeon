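; Gameplay Ability for the hero's rifle shot, dealing damage through GE_RifleDemage.
; On commit it calls the hero's PrimaryAttack and binds to the sphere overlap of the returned actor.
; Overlapping a BdCharacterBase other than the instigator applies the effect with the hit result in its context, destroys that actor and ends the ability.
; Otherwise the ability ends after a five-second delay; debug prints remain in the overlap handler.
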(event Custom|AmmoOverlap
  (params (OverlappedComponent :type Primitive%20Component%20Object%20Reference) (OtherActor :type Actor%20Object%20Reference) (OtherComp :type Primitive%20Component%20Object%20Reference) (OtherBodyIndex :type Integer) (bFromSweep :type Boolean) (SweepResult :type Hit%20Result%20Structure%20%28by%20ref%29))
  (bind _returnvalue (Ability|GetActorInfo))
  (bind (_owneractor _avataractor _playercontroller _abilitysystemcomponent) (Utilities|Struct|BreakGameplayAbilityActorInfo _returnvalue))
  (if (not (== OtherActor (Variables|/Script/Engine.Actor|GetInstigator (stale Ability|EventActivateAbility _returnvalue_2))))
    (Development|PrintString (Utilities|GetDisplayName OtherComp))
    (bind _asbd_character_base (Utilities|Casting|CastToBdCharacterBase OtherActor))
    (Development|PrintString (Utilities|GetDisplayName (Ability|GetAbilitySystemComponent _asbd_character_base)) true true "(R=0.000000,G=0.660000,B=1.000000,A=1.000000)" 1e+01)
    (bind _output_get (Variables|Default|SetContext (GameplayEffects|MakeEffectContext _abilitysystemcomponent)))
    (Class|AbilitySystemBlueprintLibrary|EffectContextAddHitResult _output_get SweepResult false)
    (GameplayEffects|ApplyGameplayEffectToTarget _abilitysystemcomponent "/Game/Weapons/Rifle/GE_RifleDemage.GE_RifleDemage_C" (Ability|GetAbilitySystemComponent _asbd_character_base) 1.0 _output_get)
    (Actor|DestroyActor (stale Ability|EventActivateAbility _returnvalue_2))
    (Ability|EndAbility)))

(event Ability|EventActivateAbility
  (bind _returnvalue (Ability|CommitAbility))
  (if _returnvalue
    (bind _asbd_character_hero (Utilities|Casting|CastToBdCharacterHero (.AvatarActor (Utilities|Struct|BreakGameplayAbilityActorInfo (Ability|GetActorInfo)))))
    (bind _returnvalue_2 (Class|BdCharacterHero|PrimaryAttack _asbd_character_hero))
    (Collision|BindEventtoOnComponentBeginOverlap (Variables|/Script/BulletDungeon.BdAmmoBase|GetSphereComponent _returnvalue_2) (delegate Custom|AmmoOverlap))
    (Utilities|FlowControl|Delay 5.0)
    (Ability|EndAbility)
    (else
      (Ability|EndAbility))))

(event Ability|EventOnEndAbility
  (params (bWasCancelled :type Boolean)))