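; BP_Recoil defines a weapon's recoil and spread through curve assets.
; Ammo index samples curves for camera pitch and yaw kick and for up and right directional spread, while time since stop samples the camera restore ratio.
; Random spread reads the same right-spread curve as directional spread.
; ApplyCameraShake takes an ammo index and controller but is empty.
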(fn GetCameraMovement
  (params (AmmoIndex :type Float%20%28single-precision%29))
  (return (Math|Curves|GetFloatValue (Variables|Default|GetPitchCurve) AmmoIndex) (Math|Curves|GetFloatValue (Variables|Default|GetYawCurve) AmmoIndex)))

(fn GetCameraRestoreRatio
  (params (TimeSinceStop :type Float%20%28single-precision%29))
  (return (Math|Curves|GetFloatValue (Variables|Default|GetCameraRestoreCurve) TimeSinceStop)))

(fn GetDirectionalSpread
  (params (AmmoIndex :type Float%20%28single-precision%29))
  (return (Math|Curves|GetFloatValue (Variables|Default|GetUpSpreadCurve) AmmoIndex) (Math|Curves|GetFloatValue (Variables|Default|GetRightSpreadCurve) AmmoIndex)))

(fn GetRandomSpread
  (params (AmmoIndex :type Float%20%28single-precision%29))
  (return (Math|Curves|GetFloatValue (Variables|Default|GetRightSpreadCurve) AmmoIndex)))

(fn ApplyCameraShake
  (params (AmmoIndex :type Float%20%28single-precision%29) (controller :type Player%20Controller%20Object%20Reference)))