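; BP_BdRifleAmmo is a rifle ammo pickup that a hero character interacts with to gain ammo.
; On interaction it marks its equipment spawn point as unspawned, then adds its own class in BaseNum quantity to the hero's InventoryComponent.
; A successful add applies the interaction effect and destroys the actor.
; Without a valid spawn point, it destroys itself without granting ammo.
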(event EventBeginPlay)

(event Collision|EventActorBeginOverlap
  (params (OtherActor :type Actor%20Object%20Reference)))

(event EventTick
  (params (DeltaSeconds :type Float%20%28single-precision%29)))

(event EventUse
  (params (Target :type Pawn%20Object%20Reference)))

(event EventInteracted
  (params (InstigatorPawn :type Pawn%20Object%20Reference))
  (bind _spawnpoint (Variables|Default|GetSpawnPoint))
  (Utilities|IsValid _spawnpoint
    (:Is%20Valid
      (bind _asbd_equipment_spawn_point (Utilities|Casting|CastToBdEquipmentSpawnPoint _spawnpoint))
      (Variables|/Script/BulletDungeon.BdEquipmentSpawnPoint|SetbIsSpawned _asbd_equipment_spawn_point false)
      (bind _asbd_character_hero (Utilities|Casting|CastToBdCharacterHero InstigatorPawn))
      (bind _returnvalue (Class|BdInventoryComponent|AddItem (Variables|/Script/BulletDungeon.BdCharacterHero|GetInventoryComponent _asbd_character_hero) "BP_BdRifleAmmo_C" (Variables|Default|GetBaseNum)))
      (if _returnvalue
        (Class|BdEquipment|InteractionEffectApply _asbd_character_hero)
        (Actor|DestroyActor :!label _label)))
    (:Is%20Not%20Valid
      (goto _label))))

(fn ConstructionScript)