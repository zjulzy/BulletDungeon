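; Demo rifle weapon that a hero character picks up by interacting with it.
; Interaction spawns a copy owned by the hero and adds it to the inventory, then attaches it to the weapon socket and destroys the original, or discards the copy on failure.
; Shooting plays the fire animation and zeroes ammo, which starts full.
; A scene capture renders only the rifle mesh; Equip is empty.
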(event EventBeginPlay
  (Variables|Default|SetAmmos (Variables|Default|GetMaxAmmos)))

(event EventEquip)

(event EventInteracted
  (params (InstigatorPawn :type Pawn%20Object%20Reference))
  (bind _self self)
  (bind _asbd_character_hero (Utilities|Casting|CastToBdCharacterHero InstigatorPawn))
  (Class|BdInventoryComponent|QueryWeapon (Variables|/Script/BulletDungeon.BdCharacterHero|GetInventoryComponent _asbd_character_hero) self)
  (if true
    (bind _returnvalue (Game|SpawnActorfromClass (Utilities|GetClass _self) (Transformation|GetActorTransform _self) "AdjustIfPossibleButAlwaysSpawn" "MultiplyWithRoot" _asbd_character_hero _asbd_character_hero))
    (bind _returnvalue_2 (Class|BdInventoryComponent|AddWeapon (Variables|/Script/BulletDungeon.BdCharacterHero|GetInventoryComponent _asbd_character_hero) _returnvalue))
    (if _returnvalue_2
      (Transformation|AttachComponentToComponent _returnvalue (Variables|/Script/Engine.Character|GetMesh _asbd_character_hero) "weapon_socket" "SnapToTarget" "SnapToTarget" "SnapToTarget" true)
      (Actor|DestroyActor)
      (else
        (Actor|DestroyActor _returnvalue)))))

(event EventShoot
  (Components|Animation|PlayAnimation (Variables|Default|GetSkeletalMeshComponent) "/Game/MilitaryWeapDark/Weapons/Anims/Fire_Rifle_W.Fire_Rifle_W" false)
  (Variables|Default|SetAmmos 0.0))

(fn ConstructionScript
  (Rendering|SceneCapture|ShowOnlyComponent (Variables|Default|GetSceneCaptureComponent2D) (Variables|Default|GetSkeletalMeshComponent)))