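; Human assault rifle gun Blueprint that fires automatically while the trigger is held.
; FireSequence loops on a retriggerable delay, spawning a projectile at the computed target transform and triggering character fire animation, crosshair and muzzle flash.
; Each shot shortens the delay and raises Spread within clamped limits, so sustained fire speeds up.
; Releasing the trigger stops the loop, then resets Spread and FireRate after a short delay.
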(event EventBeginPlay
  (|CallParentFunction)
  (Variables|Default|SetSpread 1.0))

(event EventTriggerReleased
  (Variables|Default|SetIsFiring false)
  (Utilities|FlowControl|RetriggerableDelay 0.5)
  (Variables|Default|SetSpread 0.0)
  (Variables|Default|SetFireRate 0.3))

(event EventFireSequence
  (bind _playercharacter (Variables|Default|GetPlayerCharacter))
  (Variables|Default|SetIsFiring true)
  (bind _transform (CallFunction|GetProjectileTarget 1e+04 :!label _label))
  (Game|SpawnActorfromClass "/Game/AddOn/CatalystVFX/Blueprints/Projectiles/BP_Projectile_AssaultRifle_Human.BP_Projectile_AssaultRifle_Human_C" _transform "AdjustIfPossibleButDontSpawnIfColliding" "OverrideRootScale" 0 0) ; Spawn projectile
  (Default|FireAnim _playercharacter)
  (Default|ActivateCrosshair _playercharacter)
  (Components|Activation|Activate (Variables|Default|GetMuzzleFlash) true)
  (Variables|Default|SetFireRate (Math|Float|Clamp(Float) (- (Variables|Default|GetFireRate) 0.02) 0.15))
  (Variables|Default|SetSpread (Math|Float|Clamp(Float) (+ (Variables|Default|GetSpread) 0.3) 0.0 1.3))
  (Utilities|FlowControl|RetriggerableDelay (Variables|Default|GetFireRate))
  (if (Variables|Default|GetIsFiring)
    (goto _label)))

(fn ConstructionScript
  (|CallParentFunction))