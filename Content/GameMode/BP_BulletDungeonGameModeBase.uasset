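; Game mode for Bullet Dungeon that advances the player through streamed dungeon levels as difficulty increases.
; LoadandTravelNewLevel loads a random map as a level instance at the next location, or the final map once difficulty passes the maximum, then requests unload of the previous instance.
; After a short delay it moves the player to BP_Destination, resets the game-state goal and signals a refresh.
; Calling it again after the last level opens the end map.
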(event EventBeginPlay)

(event EventTick
  (params (DeltaSeconds :type Float%20%28single-precision%29)))

(event EventLoadandTravelNewLevel
  (bind _array (Utilities|Array|MakeArray "/Game/Maps/L_DemoMap.L_DemoMap" "/Game/Maps/L_NextMap.L_NextMap"))
  (bind _returnvalue (Utilities|Array|Length _array))
  (if (Variables|Default|GetbLastLevel)
    (Game|OpenLevel(byObjectReference) "/Game/Maps/L_EndUp.L_EndUp")
    (else
      (bind _result (Math|Integer|IncrementInt (Variables|Default|GetDifficulty))
        (:%20%20
          (Variables|Default|SetbLastLevel (> _result (Variables|Default|GetMaxLevel)))
          (bind _returnvalue_2 (Class|BulletDungeonGameModeBase|GetNextLevelLocation))
          (bind _output_get (Variables|Default|SetCurrentLevelLocation _returnvalue_2))
          (if (Variables|Default|GetbLastLevel)
            (Variables|Default|SetNewVar _returnvalue)
            (Class|LevelStreamingDynamic|LoadLevelInstancebySoftObjectPtr "/Game/Maps/L_FinalMap.L_FinalMap" _output_get "0, 0, 0" "" 0 false)
            (else
              (bind _output_get_2 (Variables|Default|SetNewVar (Math|Random|RandomInteger _returnvalue)))
              (bind _returnvalue_3 (Class|LevelStreamingDynamic|LoadLevelInstancebySoftObjectPtr (Utilities|Array|Get(acopy) _array _output_get_2) _output_get "0, 0, 0" "" 0 false))))
          (if (Utilities|IsValid (Variables|Default|GetCurrentLevel))
            (Class|LevelStreaming|SetIsRequestingUnloadandRemoval (Variables|Default|GetCurrentLevel) true))
          (Variables|Default|SetCurrentLevel _returnvalue_3)
          (Utilities|FlowControl|Delay 0.2)
          (bind _returnvalue_4 (Actor|GetActorOfClass "/Game/GameMode/BP_Destination.BP_Destination_C"))
          (Transformation|SetActorLocation (Game|Player|GetPlayerPawn 0) (Transformation|GetActorLocation _returnvalue_4) false false)
          (Actor|DestroyActor _returnvalue_4)
          (bind _asbd_game_state_base (Utilities|Casting|CastToBdGameStateBase (Game|GetGameState)))
          (Class|BdGameStateBase|ResetGoal _asbd_game_state_base (Utilities|Array|Get(acopy) (Utilities|Array|MakeArray "L_DemoMap" "L_NextMap" "L_FinalMap") (Variables|Default|GetNewVar)))
          (Default|CallRefreshLevel))))))

(fn ConstructionScript)