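; Human assault rifle projectile Blueprint from CatalystVFX that handles the visual response to a hit.
; Its Hit event spawns a small Niagara explosion aligned to the surface normal, then after a brief delay deactivates the trail and hides the sphere.
; It spawns a scaled-down BP_ImpactDecal with the rifle impact material while a timeline drives the trail's manual alpha.
; The actor destroys itself after a further short delay.
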(event Collision|EventHit
  (params (MyComp :type Primitive%20Component%20Object%20Reference) (Other :type Actor%20Object%20Reference) (OtherComp :type Primitive%20Component%20Object%20Reference) (bSelfMoved :type Boolean) (HitLocation :type Vector :default "0, 0, 0") (HitNormal :type Vector :default "0, 0, 0") (NormalImpulse :type Vector :default "0, 0, 0") (Hit :type Hit%20Result%20Structure%20%28by%20ref%29))
  (bind _returnvalue (Math|Conversions|RotationFromXVector HitNormal))
  (bind _ns_rockettrail (Variables|Default|GetNS_RocketTrail))
  (Niagara|SpawnSystematLocation "/Game/AddOn/CatalystVFX/ParticleSystems/Impacts/NS_ExplosionSmall_Human.NS_ExplosionSmall_Human" HitLocation _returnvalue)
  (Utilities|FlowControl|Delay 0.1)
  (Components|Activation|Deactivate _ns_rockettrail)
  (Utilities|FlowControl|Sequence
    (:then_0
      (Rendering|SetVisibility (Variables|MyProjectile|GetSphere) false false)
      (bind _returnvalue_2 (Game|SpawnActorfromClass "/Game/AddOn/CatalystVFX/Blueprints/BP_ImpactDecal.BP_ImpactDecal_C" (Math|Transform|MakeTransform HitLocation _returnvalue "0.050000,0.050000,0.050000") "Undefined" "OverrideRootScale" 0 (Game|GetPlayerCharacter 0)))
      (Default|InitiateDecal _returnvalue_2 "/Game/AddOn/CatalystVFX/Materials/Decals/M_AssaultRifleImpact_Human.M_AssaultRifleImpact_Human" 2.0 3.0)
      (Utilities|FlowControl|Delay 0.8)
      (Actor|DestroyActor) ; Then destroy this projectile
    )
    (:then_1
      (bind _newtrack_0 (Timeline|Timeline_0 PlayFromStart)
        (:Update
          (Niagara|SetNiagaraVariable(Float) _ns_rockettrail "Particles_ManualAlpha" _newtrack_0))))))

(fn ConstructionScript)